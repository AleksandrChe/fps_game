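; BP_MainCharacter is the player character Blueprint, handling movement, camera look and sprinting through Enhanced Input.
; On BeginPlay it adds the default mapping context to the controlling player's input subsystem.
; Move input is applied along directions derived from control rotation, with forward movement using yaw only, while look input drives controller yaw and pitch.
; Sprint raises the walk speed while triggered and restores the slower speed when completed or canceled.
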(event `self.ReceiveBeginPlay`
  (bind _asplayer_controller (cast `PlayerController` (`self.GetController`)))
  (`EnhancedInputSubsystemInterface.AddMappingContext` (pcsubsystem `EnhancedInputLocalPlayerSubsystem` _asplayer_controller) "/Game/Data/Inputs/IMC_Default.IMC_Default" 0 (struct)))

(event `EnhancedInput|/Game/Data/Inputs/IA_Move`
  (params (ActionValue :type "Vector2D Structure") (ElapsedSeconds :type "Float (double-precision)") (TriggeredSeconds :type "Float (double-precision)") (InputAction :type "InputAction Object Reference" :default "/Game/Data/Inputs/IA_Move.IA_Move"))
  (bind (_returnvalue_roll _returnvalue_pitch _returnvalue_yaw) (`KismetMathLibrary.BreakRotator` (`self.GetControlRotation`)))
  (bind (_returnvalue_roll_2 _returnvalue_pitch_2 _returnvalue_yaw_2) (`KismetMathLibrary.BreakRotator` (`self.GetControlRotation`)))
  ; Move Character
  (:`Triggered`
    ;; Move Left/Right
    (`self.AddMovementInput` (`KismetMathLibrary.GetRightVector` (`KismetMathLibrary.MakeRotator` _returnvalue_roll 0.0 _returnvalue_yaw)) ActionValue_X)
    ;; Move Forward/Back
    (`self.AddMovementInput` (`KismetMathLibrary.GetForwardVector` (`KismetMathLibrary.MakeRotator` 0.0 0.0 _returnvalue_yaw_2)) ActionValue_Y)))

(event `EnhancedInput|/Game/Data/Inputs/IA_Look`
  (params (ActionValue :type "Vector2D Structure") (ElapsedSeconds :type "Float (double-precision)") (TriggeredSeconds :type "Float (double-precision)") (InputAction :type "InputAction Object Reference" :default "/Game/Data/Inputs/IA_Look.IA_Look"))
  ; Camera
  (:`Triggered`
    ;; Camera Left/Right
    (`self.AddControllerYawInput` ActionValue_X)
    ;; Camera Up/Down
    (`self.AddControllerPitchInput` ActionValue_Y)))

(event `EnhancedInput|/Game/Data/Inputs/IA_Sprint`
  (params (ActionValue :type Boolean) (ElapsedSeconds :type "Float (double-precision)") (TriggeredSeconds :type "Float (double-precision)") (InputAction :type "InputAction Object Reference" :default "/Game/Data/Inputs/IA_Sprint.IA_Sprint"))
  (bind _charactermovement (`self.CharacterMovement`))
  ; Walk/Run
  (:`Triggered`
    (set `CharacterMovementComponent.MaxWalkSpeed` 400.0 _charactermovement))
  (:`Canceled`
    (set `CharacterMovementComponent.MaxWalkSpeed` 200.0 _charactermovement :!label _label))
  (:`Completed`
    (goto _label)))

(fn `UserConstructionScript`)